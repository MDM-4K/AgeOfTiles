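; RTS player controller that drives the camera pawn, handles selection and creates the main HUD.
; BeginPlay centers the camera, pushes data-table resources to the HUD and spawns a Viking Town Centre at a ground-traced start location.
; Axis input pans at zoom-scaled speed, screen edges scroll, and zoom adjusts spring arm length.
; Cursor traces select the Town Centre or, when gated on, track landscape position; debug keys send unit-selection messages to the HUD.
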(event `self.ReceiveBeginPlay`
  (`|ExecutionSequence`
    (:`then_0`
      ;[1 1 1] Set References
      (`|ExecutionSequence`
        (:`then_0`
          (`self.SetReferences`))
        (:`then_1`
          (`self.Set CameraFirstPosition`))))
    (:`then_1`
      (`UserWidget.AddToViewport` (`self.MainPlayerHudRef`) 0))
    (:`then_2`
      (`self.SetInitialResources`)
      (`self.UpdateResources`))
    (:`then_3`
      (`self.SetPlayerSpawnLocation`)
      (`|SpawnActorFromClass` "/Game/AgeofTiles/Buildings/Economy/TownCentre/Vikings/TownCentreViking_Child3.TownCentreViking_Child3_C" (`KismetMathLibrary.MakeTransform` (`self.PlayerSpawnLocation`)) "Undefined" "OverrideRootScale" null null "TownCentre" (struct) null))))

(event `Key|V`
  (params (Key :type "Key Structure"))
  (:`Pressed`
    (message `/Game/AgeofTiles/Interfaces/Unit_Interface.Testing_Testing` (`self.MainPlayerHudRef`))))

(event `InputAxis|MoveForward`
  (params (AxisValue :type "Float (single-precision)"))
  (bind _camerapawnreference (`self.CameraPawnReference`))
  ;[1 1 1] Camera Movement
  (if (not (`self.DisableCamNav`))
    (`self.K2_SetActorTransform` _camerapawnreference (`self.MovementX` AxisValue (`self.MovementSpeedCalculation`) (`self.FastMoveMultiplier`) _camerapawnreference) false false)))

(event `Pause_Game`
  ;[1 1 1] Pause Game
  (`self.PauseGame`))

(event `InputAxis|MoveRight`
  (params (AxisValue :type "Float (single-precision)"))
  (bind _camerapawnreference (`self.CameraPawnReference`))
  ;[1 1 1] Camera Movement
  (if (not (`self.DisableCamNav`))
    (`self.K2_SetActorTransform` _camerapawnreference (`self.MovementY` AxisValue (`self.MovementSpeedCalculation`) (`self.FastMoveMultiplier`) _camerapawnreference) false false)))

(event `Resume_Game`
  ;[1 1 1] Resume Game
  (`self.ResumeGame`))

(event `InputAction|ZoomIn`
  (params (Key :type "Key Structure"))
  (bind _springarm (`/Game/AgeofTiles/Blueprints/CameraPawn.SpringArm` (`self.CameraPawnReference`)))
  ;[1 1 1] Zooming
  (:`Pressed`
    (set `SpringArmComponent.TargetArmLength` (`KismetMathLibrary.FClamp` (- (`SpringArmComponent.TargetArmLength` _springarm) (`self.ZoomSensativity`)) 500.0 (`self.MaxArmDistance`)) _springarm)))

(event `InputAction|ZoomOut`
  (params (Key :type "Key Structure"))
  (bind _springarm (`/Game/AgeofTiles/Blueprints/CameraPawn.SpringArm` (`self.CameraPawnReference`)))
  ;[1 1 1] Zooming
  (:`Pressed`
    (set `SpringArmComponent.TargetArmLength` (`KismetMathLibrary.FClamp` (+ (`SpringArmComponent.TargetArmLength` _springarm) (`self.ZoomSensativity`)) 500.0 (`self.MaxArmDistance`)) _springarm)))

(event `InputAxisKey|MouseX`
  (params (AxisValue :type "Float (single-precision)"))
  ;[1 1 1] EdgeScroll
  (if (not (`self.DisableCamNav`))
    (bind (_deltaxspeed _deltayspeed) (`self.ScreenEdgeMovement` :!label _label))
    (`self.K2_AddActorLocalOffset` (`self.CameraPawnReference`) (`KismetMathLibrary.MakeVector` _deltaxspeed _deltayspeed) true false)))

(event `InputAxisKey|MouseY`
  (params (AxisValue :type "Float (single-precision)"))
  ;[1 1 1] EdgeScroll
  (if (not (`self.DisableCamNav`))
    (goto _label :!via `MouseY`)))

(event `InputAction|PrimaryMouseBtn`
  (params (Key :type "Key Structure"))
  (bind (_worldlocation _worlddirection) (`self.DeprojectMousePositionToWorld` (`GameplayStatics.GetPlayerController` (`self.PlayerIndex`))))
  (:`Pressed`
    (bind _outhit (`KismetSystemLibrary.LineTraceSingle` (`SceneComponent.K2_GetComponentLocation` (`/Game/AgeofTiles/Blueprints/CameraPawn.Camera` (`self.CameraPawnReference`))) (+ _worldlocation (* _worlddirection 50000.0)) "TraceTypeQuery4"))
    (bind _astown_centre_viking_child_3 (cast `/Game/AgeofTiles/Buildings/Economy/TownCentre/Vikings/TownCentreViking_Child3` (`.HitActor` (`GameplayStatics.BreakHitResult` _outhit)))
      (:`then`
        (set `self.SelectedBuilding` _astown_centre_viking_child_3)
        (`self.SelectBuilding` "TownCentre"))
      (:`CastFailed`
        (`self.DeSelect`)))))

(event `Key|R`
  (params (Key :type "Key Structure"))
  (:`Pressed`
    (`self.UpdateResources`)))

(event `Key|Zero`
  (params (Key :type "Key Structure"))
  ;[1 1 1] Deselect
  (:`Pressed`
    (`self.DeSelect`)))

(event `Key|One`
  (params (Key :type "Key Structure"))
  ;[1 1 1] Select Buildings
)

(event `Key|Two`
  (params (Key :type "Key Structure"))
  ;[1 1 1] Select Buildings
)

(event `Key|Three`
  (params (Key :type "Key Structure"))
  ;[1 1 1] Select Buildings
)

(event `Key|Four`
  (params (Key :type "Key Structure"))
  ;[1 1 1] Select Buildings
)

(event `Key|Five`
  (params (Key :type "Key Structure"))
  ;[1 1 1] Select Buildings
)

(event `Key|Six`
  (params (Key :type "Key Structure"))
  ;[1 1 1] Select Buildings
)

(event `Key|Seven`
  (params (Key :type "Key Structure"))
  ;[1 1 1] Select Buildings
  (:`Pressed`
    (`self.SelectUnits` :!label _label_2)))

(event `Key|Eight`
  (params (Key :type "Key Structure"))
  ;[1 1 1] Select Buildings
  (:`Pressed`
    (goto _label_2 :!via `SelectRangedUnit1`)))

(event `Key|Nine`
  (params (Key :type "Key Structure"))
  ;[1 1 1] Select Buildings
  (:`Pressed`
    (goto _label_2 :!via `SelectMeleeUnit1`)))

(event `InputAxisKey|MouseX`
  (params (AxisValue :type "Float (single-precision)"))
  (`/Engine/EditorBlueprintResources/StandardMacros.Gate` true :!label _label_3
    (:`Exit`
      (`self.GetMouseLandscapeHitLocation`))))

(event `InputAxisKey|MouseY`
  (params (AxisValue :type "Float (single-precision)"))
  (goto _label_3))

(event `ToggleGetMouseLocationOn`
  (goto _label_3 :!via `Open`))

(event `ToggleGetMouseLocationOff`
  (goto _label_3 :!via `Close`))

(fn `ClickSelectableBuilding`
  (returns (OutHit_HitActor :type "Actor Object Reference"))
  (bind (_worldlocation _worlddirection) (`self.DeprojectMousePositionToWorld` (`GameplayStatics.GetPlayerController` (`self.PlayerIndex`))))
  (bind (_outhit _returnvalue) (`KismetSystemLibrary.LineTraceSingle` :`Start` (`SceneComponent.K2_GetComponentLocation` (`/Game/AgeofTiles/Blueprints/CameraPawn.Camera` (`self.CameraPawnReference`))) :`End` (+ _worldlocation (* _worlddirection 50000.0)) :`TraceChannel` "TraceTypeQuery4" :`DrawDebugType` "Persistent"))
  (if _returnvalue
    (return (`.HitActor` (`GameplayStatics.BreakHitResult` _outhit)))))

(fn `DeSelect`
  (message `/Game/AgeofTiles/Interfaces/Unit_Interface.De_Select` (`self.MainPlayerHudRef`)))

(fn `GetMouseLandscapeHitLocation`
  (bind (_worldlocation _worlddirection) (`self.DeprojectMousePositionToWorld` (`GameplayStatics.GetPlayerController` (`self.PlayerIndex`))))
  (bind (_outhit _returnvalue) (`KismetSystemLibrary.LineTraceSingle` (`SceneComponent.K2_GetComponentLocation` (`/Game/AgeofTiles/Blueprints/CameraPawn.Camera` (`self.CameraPawnReference`))) (+ _worldlocation (* _worlddirection 50000.0)) "TraceTypeQuery3"))
  (if _returnvalue
    (bind _output_get (set `self.CursorLanscapeLocation` (`.Location` (`GameplayStatics.BreakHitResult` _outhit))))
    (`KismetSystemLibrary.PrintString` (`KismetStringLibrary.Conv_VectorToString` _output_get))
    (else
      (bind _output_get_2 (set `self.CursorLanscapeLocation` (`.TraceEnd` (`GameplayStatics.BreakHitResult` _outhit))))
      (`KismetSystemLibrary.PrintString` (`KismetStringLibrary.Conv_VectorToString` _output_get_2))))
  (return))

(fn `MovementSpeedCalculation`
  (returns (ReturnValue :type "Float (double-precision)"))
  (return (`KismetMathLibrary.FClamp` (/ (`SpringArmComponent.TargetArmLength` (`/Game/AgeofTiles/Blueprints/CameraPawn.SpringArm` (`self.CameraPawnReference`))) 100.0) 5.0 20.0)))

(fn `PauseGame`
  (`self.DisableInput` (`GameplayStatics.GetPlayerController` 0))
  (return))

(fn `ResumeGame`
  (`self.EnableInput` (`GameplayStatics.GetPlayerController` 0))
  (return))

(fn `SelectBuilding`
  (params (Building :type Name))
  (message `/Game/AgeofTiles/Interfaces/Unit_Interface.Select_Building` (`self.MainPlayerHudRef`) Building))

(fn `SetInitialResources`)

(fn `UpdateResources`
  (bind _outrownames (`DataTableFunctionLibrary.GetDataTableRowNames` "/Game/AgeofTiles/DataTables/Resources_Data.Resources_Data"))
  (for _array_element _outrownames
    (bind _returnvalue (`|GetDataTableRow` "/Game/AgeofTiles/DataTables/Resources_Data.Resources_Data" _array_element)
      (:`then`
        (message `/Game/AgeofTiles/Interfaces/Unit_Interface.Update_Resources` (`self.MainPlayerHudRef`) _returnvalue)
        (return)))))

(fn `UserConstructionScript`)