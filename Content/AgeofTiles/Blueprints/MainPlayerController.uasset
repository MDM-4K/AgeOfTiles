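; RTS player controller that sets up HUD, resources and a starting Town Centre, then handles camera, building and unit commands.
; Data table rows drive building and Worker spawns, with gates making placement ghosts follow the cursor on a grid until clicked.
; Channel-specific cursor traces select buildings or units, with shift-toggle and double-click select-all.
; Right-click moves units or the building's rally marker; box selection and formation marker spawning are unwired.
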(event `self.ReceiveBeginPlay`
  ;[1 1 1] BeginPlay
  (`|ExecutionSequence`
    (:`then_0`
      ;[1 1 1] Set References
      (`|ExecutionSequence`
        (:`then_0`
          (`self.SetReferences`))
        (:`then_1`
          (`self.Set CameraFirstPosition`))))
    (:`then_1`
      (`UserWidget.AddToViewport` (`self.MainPlayerHudRef`) 0)
      (`self.SetInitialResources` (make `/Game/AgeofTiles/Structs/Resources_Struct` 50 50 50 50 50 50 0 50 1 1)))
    (:`then_3`
      (`self.SetPlayerSpawnLocation`))
    (:`then_4`
      ;[1 1 1] Spawn Initial Building
      (bind _returnvalue (`|GetDataTableRow` "/Game/AgeofTiles/DataTables/Buildings_Data.Buildings_Data" "TownCentre")
        (:`then`
          (bind _returnvalue_2 (`|SpawnActorFromClass` "/Game/AgeofTiles/Buildings/TownCentre.TownCentre_C" (`KismetMathLibrary.MakeTransform` (`self.PlayerSpawnLocation`)) "Undefined" "OverrideRootScale" null self _returnvalue (`self.MainPlayerHudRef`) null))
          (message `/Game/AgeofTiles/Interfaces/PlayerMainHUD_Interface.Create_Building_Widget` (`self.MainPlayerHudRef`) _returnvalue_2 "NewEnumerator0")
          (`self.SelectBuilding` _returnvalue_2 "NewEnumerator0"))))))

(event `Resume_Game`
  ;[1 1 1] Resume Game
  (`self.ResumeGame`))

(event `Key|LeftShift`
  (params (Key :type "Key Structure"))
  ;[1 1 1] LeftShift
  (:`Pressed`
    (set `self.LeftShiftPressed` true))
  (:`Released`
    (set `self.LeftShiftPressed` false)))

(event `Pause_Game`
  ;[1 1 1] Pause Game
  (`self.PauseGame`))

(event `InputAxisKey|MouseX`
  (params (AxisValue :type "Float (single-precision)"))
  (bind (_cursorlanscapelocation_x _cursorlanscapelocation_y _cursorlanscapelocation_z) (`KismetMathLibrary.BreakVector` (`self.CursorLanscapeLocation`)))
  (bind _gridsize (`self.GridSize`))
  (`/Engine/EditorBlueprintResources/StandardMacros.Gate` true :!label _label
    (:`Exit`
      (bind (_outhit _returnvalue) (`self.GetMouseHitLocation` "TraceTypeQuery3"))
      (if _returnvalue
        (set `self.CursorLanscapeLocation` (`.Location` (`GameplayStatics.BreakHitResult` _outhit)))
        (else
          (set `self.CursorLanscapeLocation` (`.TraceEnd` (`GameplayStatics.BreakHitResult` _outhit)))))
      (`self.K2_SetActorLocation` (stale `/Game/AgeofTiles/Interfaces/PlayerController_Interface.Spawn_Building` _returnvalue_2) (`KismetMathLibrary.MakeVector` (`/Game/AgeofTiles/Libraries/FunctionLibrary/Calculations.Grid` _cursorlanscapelocation_x _gridsize) (`/Game/AgeofTiles/Libraries/FunctionLibrary/Calculations.Grid` _cursorlanscapelocation_y _gridsize) _cursorlanscapelocation_z) false false))))

(event `InputAxisKey|MouseY`
  (params (AxisValue :type "Float (single-precision)"))
  (goto _label))

(event `/Game/AgeofTiles/Interfaces/PlayerController_Interface.Spawn_Building`
  (params (BuildingName :type Name) (TargetButton :type "Widget Object Reference"))
  ;[1 1 1] Spawn Building
  (bind _returnvalue (`|GetDataTableRow` "/Game/AgeofTiles/DataTables/Buildings_Data.Buildings_Data" BuildingName)
    (:`then`
      (bind _returnvalue_2 (`|SpawnActorFromClass` "/Game/AgeofTiles/Buildings/TownCentre.TownCentre_C" (`KismetMathLibrary.MakeTransform` (0.0 0.0 0.0)) "Undefined" "OverrideRootScale" null null _returnvalue null null))
      (message `/Game/AgeofTiles/Interfaces/PlayerMainHUD_Interface.Create_Building_Widget` (`self.MainPlayerHudRef`) _returnvalue_2 (`.Name_69_DCFE0DCD41D014C9A532C3802843C705` (break `/Game/AgeofTiles/Structs/Building_Struct` _returnvalue)))
      (`|ExecutionSequence`
        (:`then_0`
          (goto _label :!via `Open`))
        (:`then_1`
          (set `self.BuildingPlaceMode` true)
          (goto _label_2 :!via `Open`))))
    (:`RowNotFound`
      (`KismetSystemLibrary.PrintString` "Building Row Not Found" true true (struct :`R` 1.0 :`G` 0.050025 :`B` 0.109751 :`A` 1.0)))))

(event `InputAction|PrimaryMouseBtn`
  (params (Key :type "Key Structure"))
  ;[1 1 1] PrimaryMouse
  (:`Pressed`
    (set `self.AmountOfClicks` (+ (`self.AmountOfClicks`) 1))
    (`|ExecutionSequence`
      (:`then_2`
        (if (`self.BuildingPlaceMode`)
          (set `self.BuildingPlaceMode` false)
          (`|ExecutionSequence`
            (:`then_0`
              (goto _label :!via `Close`))
            (:`then_1`
              (`/Engine/EditorBlueprintResources/StandardMacros.Gate` true :!label _label_2
                (:`Exit`
                  (`self.BuildingPlaced` (stale `/Game/AgeofTiles/Interfaces/PlayerController_Interface.Spawn_Building` TargetButton))
                  (goto _label_2 :!via `Close`)))))
          (else
            (`|ExecutionSequence`
              (:`then_0`
                (`self.SelectSomething`))))))))
  (:`Released`
    (`KismetSystemLibrary.Delay` 0.2)
    (set `self.AmountOfClicks` 0)))

(event `/Game/AgeofTiles/Interfaces/PlayerController_Interface.Spawn_Unit`
  (params (Building :type "/Game/AgeofTiles/Buildings/TownCentre Object Reference"))
  ;[1 1 1] Spawn Unit
  (bind _returnvalue (`|GetDataTableRow` "/Game/AgeofTiles/DataTables/Units_Data.Units_Data" "Worker")
    (:`then`
      (bind _structout (setmembers `/Game/AgeofTiles/Structs/Units_Struct` :`StructRef` _returnvalue))
      (bind _returnvalue_2 (`|SpawnActorFromClass` "/Game/AgeofTiles/Units/Worker_Unit.Worker_Unit_C" (`KismetMathLibrary.MakeTransform` (`SceneComponent.K2_GetComponentLocation` (`/Game/AgeofTiles/Buildings/Building_Master.UnitSpawn` Building))) "Undefined" "OverrideRootScale" null Building _structout null))
      (message `/Game/AgeofTiles/Interfaces/Unit_Master_Interface.MoveTo` _returnvalue_2 (+ (`SceneComponent.K2_GetComponentLocation` (`/Game/AgeofTiles/Buildings/Building_Master.Marker` Building)) (* (`KismetMathLibrary.RandomUnitVector`) (`KismetMathLibrary.RandomFloatInRangeFromStream` 80.0 500.0 (`KismetMathLibrary.MakeRandomStream` 0))))))))

(event `Key|Subtract`
  (params (Key :type "Key Structure"))
  (:`Pressed`
    (for _array_element (`self.SelectedUnits`)
      (`/Game/AgeofTiles/Units/Unit_Master.TakeDamage` _array_element 5))))

(event `SetBuildingMarkerEvent`
  (bind (_start _end) (`self.GetMouseStartandEndTraceLocation` (`self.PlayerIndex`)))
  ;[1 1 1] Set Building Marker
  (bind (_outhit _returnvalue) (`KismetSystemLibrary.LineTraceSingle` :`Start` _start :`End` _end :`TraceChannel` "TraceTypeQuery3" :`DrawDebugType` "Persistent"))
  (if _returnvalue
    (`self.SetBuildingMarker` (`self.SelectedBuilding`) (`.Location` (`GameplayStatics.BreakHitResult` _outhit)))))

(event `InputAction|SecondaryMouseBtn`
  (params (Key :type "Key Structure"))
  (bind _selectedunits (`self.SelectedUnits`))
  (bind (_start _end) (`self.GetMouseStartandEndTraceLocation` (`self.PlayerIndex`)))
  ;[1 1 1] RightMouse
  (:`Pressed`
    (if (not (`self.BuildingSelected?`))
      (`|ExecutionSequence`
        (:`then_0`)
        (:`then_1`
          (bind _outhit (`self.GetMouseHitLocation` "TraceTypeQuery1"))))))
  (:`Released`
    (if (`self.BuildingSelected?`)
      (`self.SetBuildingMarkerEvent`)
      (else
        (`|ExecutionSequence`
          (:`then_0`
            (`|ExecutionSequence`))
          (:`then_1`
            (if (>= (`KismetArrayLibrary.Array_Length` _selectedunits) 0)
              (for _array_element _selectedunits
                (message `/Game/AgeofTiles/Interfaces/Unit_Master_Interface.MoveTo` _array_element (`.Location` (`GameplayStatics.BreakHitResult` _outhit))))))
          (:`then_2`
            (goto _label_3 :!via `Close`)))))))

(event `InputAxisKey|MouseX`
  (params (AxisValue :type "Float (single-precision)")))

(event `InputAxisKey|MouseY`
  (params (AxisValue :type "Float (single-precision)")))

(event `InputAxisKey|MouseX`
  (params (AxisValue :type "Float (single-precision)"))
  (bind (_start _end) (`self.GetMouseStartandEndTraceLocation` (`self.PlayerIndex`)))
  (`/Engine/EditorBlueprintResources/StandardMacros.Gate` true :!label _label_3
    (:`Exit`
      (bind _outhit (`KismetSystemLibrary.LineTraceSingle` _start _end "TraceTypeQuery3"))
      (for (_array_element _array_index) (`self.MovementPointMarkers`)
        (bind _movepoint (`/Game/AgeofTiles/Libraries/FunctionLibrary/Calculations.CalculateMovePoints` _array_index 5 0.0 (`.Location` (`GameplayStatics.BreakHitResult` (stale `InputAction|SecondaryMouseBtn` _outhit)))))
        (`self.K2_SetActorLocation` _array_element _movepoint false true)))))

(event `InputAxisKey|MouseY`
  (params (AxisValue :type "Float (single-precision)"))
  (goto _label_3))

(event `InputAxis|MoveForward`
  (params (AxisValue :type "Float (single-precision)"))
  (bind _camerapawnreference (`self.CameraPawnReference`))
  ;[1 1 1] Camera Movement
  (if (not (`self.DisableCamNav`))
    (`self.K2_SetActorTransform` _camerapawnreference (`self.MovementX` AxisValue (`self.MovementSpeedCalculation`) (`self.FastMoveMultiplier`) _camerapawnreference) false false)))

(event `InputAxis|MoveRight`
  (params (AxisValue :type "Float (single-precision)"))
  (bind _camerapawnreference (`self.CameraPawnReference`))
  ;[1 1 1] Camera Movement
  (if (not (`self.DisableCamNav`))
    (`self.K2_SetActorTransform` _camerapawnreference (`self.MovementY` AxisValue (`self.MovementSpeedCalculation`) (`self.FastMoveMultiplier`) _camerapawnreference) false false)))

(event `InputAction|ZoomIn`
  (params (Key :type "Key Structure"))
  (bind _springarm (`/Game/AgeofTiles/Blueprints/CameraPawn.SpringArm` (`self.CameraPawnReference`)))
  ;[1 1 1] Zooming
  (:`Pressed`
    (set `SpringArmComponent.TargetArmLength` (`KismetMathLibrary.FClamp` (- (`SpringArmComponent.TargetArmLength` _springarm) (`self.ZoomSensativity`)) -2000.0 (`self.MaxArmDistance`)) _springarm)))

(event `InputAction|ZoomOut`
  (params (Key :type "Key Structure"))
  (bind _springarm (`/Game/AgeofTiles/Blueprints/CameraPawn.SpringArm` (`self.CameraPawnReference`)))
  ;[1 1 1] Zooming
  (:`Pressed`
    (set `SpringArmComponent.TargetArmLength` (`KismetMathLibrary.FClamp` (+ (`SpringArmComponent.TargetArmLength` _springarm) (`self.ZoomSensativity`)) -2000.0 (`self.MaxArmDistance`)) _springarm)))

(event `InputAxisKey|MouseX`
  (params (AxisValue :type "Float (single-precision)"))
  ;[1 1 1] EdgeScroll
  (if (not (`self.DisableCamNav`))
    (bind (_deltaxspeed _deltayspeed) (`self.ScreenEdgeMovement` :!label _label))
    (`self.K2_AddActorLocalOffset` (`self.CameraPawnReference`) (`KismetMathLibrary.MakeVector` _deltaxspeed _deltayspeed) true false)))

(event `InputAxisKey|MouseY`
  (params (AxisValue :type "Float (single-precision)"))
  ;[1 1 1] EdgeScroll
  (if (not (`self.DisableCamNav`))
    (goto _label :!via `MouseY`)))

(event `Key|Divide`
  (params (Key :type "Key Structure"))
  ;[1 1 1] DisableCamNav
  (:`Pressed`
    (`/Engine/EditorBlueprintResources/StandardMacros.FlipFlop`
      (:`A`
        (set `self.DisableCamNav` false))
      (:`B`
        (set `self.DisableCamNav` true)))))

(fn `BuildingPlaced`
  (params (Widget :type "Widget Object Reference"))
  (message `/Game/AgeofTiles/Interfaces/MainBuildButtons_Interface.Building_Placed` Widget))

(fn `ClickSelectableBuilding`
  (returns (OutHit_HitActor :type "Actor Object Reference"))
  (bind (_worldlocation _worlddirection) (`self.DeprojectMousePositionToWorld` (`GameplayStatics.GetPlayerController` (`self.PlayerIndex`))))
  (bind (_outhit _returnvalue) (`KismetSystemLibrary.LineTraceSingle` :`Start` (`SceneComponent.K2_GetComponentLocation` (`/Game/AgeofTiles/Blueprints/CameraPawn.Camera` (`self.CameraPawnReference`))) :`End` (+ _worldlocation (* _worlddirection 50000.0)) :`TraceChannel` "TraceTypeQuery4" :`DrawDebugType` "Persistent"))
  (if _returnvalue
    (return (`.HitActor` (`GameplayStatics.BreakHitResult` _outhit)))))

(fn `CreateSelectionBox`
  (params (StartLocation :type "Vector Structure") (EndLocation :type "Vector Structure"))
  (`KismetSystemLibrary.BoxTraceSingle` :`Start` (`KismetMathLibrary.MakeVector` (.x StartLocation) (.y StartLocation) (- (.z StartLocation) 500.0)) :`End` (`KismetMathLibrary.MakeVector` (.x EndLocation) (.y EndLocation) (+ (.z EndLocation) 500.0)) :`HalfSize` (/ (- EndLocation StartLocation) 2.0) :`TraceChannel` "TraceTypeQuery3" :`DrawDebugType` "Persistent"))

(fn `DeSelectBuilding`
  (message `/Game/AgeofTiles/Interfaces/PlayerMainHUD_Interface.Deselect_Building` (`self.MainPlayerHudRef`))
  (set `self.BuildingSelected?` false)
  (`SceneComponent.SetVisibility` (`/Game/AgeofTiles/Buildings/Building_Master.Marker` (`self.SelectedBuilding`)) false false)
  (return))

(fn `DeSelectUnits`
  (`KismetArrayLibrary.Array_Clear` (`self.SelectedUnits`))
  (bind _outactors (`GameplayStatics.GetAllActorsOfClass` "/Game/AgeofTiles/Units/Unit_Master.Unit_Master_C"))
  (for _array_element _outactors
    (message `/Game/AgeofTiles/Interfaces/Unit_Master_Interface.DeSelect_Unit` _array_element)))

(fn `GetMouseHitLocation`
  (params (TraceChannel :type "ETraceTypeQuery Enum" :default "TraceTypeQuery1"))
  (returns (OutHit :type "HitResult Structure") (ReturnValue :type Boolean))
  (bind (_start _end) (`self.GetMouseStartandEndTraceLocation` (`self.PlayerIndex`)))
  (bind (_outhit _returnvalue) (`KismetSystemLibrary.LineTraceSingle` :`Start` _start :`End` _end :`TraceChannel` TraceChannel :`DrawDebugType` "Persistent"))
  (return _outhit _returnvalue))

(fn `GetMouseStartandEndTraceLocation`
  (params (PlayerIndex :type Integer))
  (returns (Start :type "Vector Structure") (End :type "Vector Structure"))
  (bind (_worldlocation _worlddirection) (`self.DeprojectMousePositionToWorld` (`GameplayStatics.GetPlayerController` PlayerIndex)))
  (return (`SceneComponent.K2_GetComponentLocation` (`/Game/AgeofTiles/Blueprints/CameraPawn.Camera` (`self.CameraPawnReference`))) (+ _worldlocation (* _worlddirection 50000.0))))

(fn `MovementSpeedCalculation`
  (returns (ReturnValue :type "Float (double-precision)"))
  (return (`KismetMathLibrary.FClamp` (/ (`SpringArmComponent.TargetArmLength` (`/Game/AgeofTiles/Blueprints/CameraPawn.SpringArm` (`self.CameraPawnReference`))) 100.0) 5.0 20.0)))

(fn `PauseGame`
  (`self.DisableInput` (`GameplayStatics.GetPlayerController` 0))
  (return))

(fn `ResumeGame`
  (`self.EnableInput` (`GameplayStatics.GetPlayerController` 0))
  (return))

(fn `SelectBuilding`
  (params (Actor :type "Actor Object Reference") (Building :type "/Game/AgeofTiles/Enumerators/Buildings_Enum Enum" :default "NewEnumerator0"))
  (bind _astown_centre (cast `/Game/AgeofTiles/Buildings/TownCentre` Actor)
    (:`then`
      (bind _output_get (set `self.SelectedBuilding` _astown_centre))
      (`self.DeSelectBuilding`)
      (message `/Game/AgeofTiles/Interfaces/PlayerMainHUD_Interface.Select_Building` (`self.MainPlayerHudRef`) Actor Building)
      (set `self.BuildingSelected?` true)
      (`SceneComponent.SetVisibility` (`/Game/AgeofTiles/Buildings/Building_Master.Marker` _output_get) true false)
      (return))
    (:`CastFailed`
      (`self.DeSelectBuilding`))))

(fn `SelectSomething`
  (bind (_start _end) (`self.GetMouseStartandEndTraceLocation` (`self.PlayerIndex`)))
  (bind (_start_2 _end_2) (`self.GetMouseStartandEndTraceLocation` (`self.PlayerIndex`)))
  (bind (_start_3 _end_3) (`self.GetMouseStartandEndTraceLocation` (`self.PlayerIndex`)))
  (`self.DeSelectBuilding`)
  (bind (_outhit _returnvalue) (`KismetSystemLibrary.LineTraceSingle` _start _end "TraceTypeQuery4"))
  (if _returnvalue
    (bind _astown_centre (cast `/Game/AgeofTiles/Buildings/TownCentre` (`.HitActor` (`GameplayStatics.BreakHitResult` _outhit))))
    (set `self.SelectedBuilding` _astown_centre)
    (`self.SelectBuilding` (`.HitActor` (`GameplayStatics.BreakHitResult` _outhit)) "NewEnumerator0")
    (`self.DeSelectUnits`)
    (else
      (`self.DeSelectBuilding`)
      (bind (_outhit_2 _returnvalue_2) (`KismetSystemLibrary.LineTraceSingle` _start_3 _end_3 "TraceTypeQuery5"))
      (if _returnvalue_2
        (bind _asworker_unit (cast `/Game/AgeofTiles/Units/Worker_Unit` (`.HitActor` (`GameplayStatics.BreakHitResult` _outhit_2))))
        (`self.SelectUnit` _asworker_unit (`self.LeftShiftPressed`))
        (else
          (`self.DeSelectUnits`)
          (`KismetSystemLibrary.LineTraceSingle` _start_2 _end_2 "TraceTypeQuery5"))))))

(fn `SelectUnit`
  (params (Actor :type "/Game/AgeofTiles/Units/Unit_Master Object Reference") (leftShiftPressed :type Boolean))
  (bind _selectedunits (`self.SelectedUnits`))
  (bind _selectedunits_2 (`self.SelectedUnits`))
  (if (== (`self.AmountOfClicks`) 2)
    (`self.DeSelectUnits`)
    (bind _outactors (`GameplayStatics.GetAllActorsOfClass` (`GameplayStatics.GetObjectClass` Actor)))
    (`KismetArrayLibrary.Array_Clear` _selectedunits)
    (for _array_element _outactors
      (bind _asunit_master (cast `/Game/AgeofTiles/Units/Unit_Master` _array_element))
      (`KismetArrayLibrary.Array_Add` _selectedunits _asunit_master)
      (message `/Game/AgeofTiles/Interfaces/Unit_Master_Interface.Select_Unit` _array_element))
    (elif leftShiftPressed
      (if (not (`KismetArrayLibrary.Array_Contains` _selectedunits_2 Actor))
        (`KismetArrayLibrary.Array_Add` _selectedunits_2 Actor)
        (message `/Game/AgeofTiles/Interfaces/Unit_Master_Interface.Select_Unit` Actor)
        (else
          (`KismetArrayLibrary.Array_RemoveItem` _selectedunits_2 Actor)
          (message `/Game/AgeofTiles/Interfaces/Unit_Master_Interface.DeSelect_Unit` Actor)))
      (else
        (`self.DeSelectUnits`)
        (`KismetArrayLibrary.Array_Add` (`self.SelectedUnits`) Actor)
        (message `/Game/AgeofTiles/Interfaces/Unit_Master_Interface.Select_Unit` Actor)))))

(fn `SetBuildingMarker`
  (params (SelectedBuilding :type "/Game/AgeofTiles/Buildings/Building_Master Object Reference") (MarkerLocation :type "Vector Structure"))
  (`SceneComponent.K2_SetWorldLocation` (`/Game/AgeofTiles/Buildings/Building_Master.Marker` SelectedBuilding) MarkerLocation false false))

(fn `SetInitialResources`
  (params (Resources :type "/Game/AgeofTiles/Structs/Resources_Struct Structure"))
  (set `self.Resources` Resources)
  (`self.UpdateResources` (`self.Resources`))
  (return))

(fn `UpdateResources`
  (params (Resources :type "/Game/AgeofTiles/Structs/Resources_Struct Structure"))
  (message `/Game/AgeofTiles/Interfaces/PlayerMainHUD_Interface.Update_Resources` (`self.MainPlayerHudRef`) Resources)
  (return))

(fn `UserConstructionScript`)